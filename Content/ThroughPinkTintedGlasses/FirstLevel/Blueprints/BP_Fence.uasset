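; BP_Fence is a procedural fence actor for the first level, built along its local Y axis.
; The construction script repeats SectionsCount sections, each a pillar instance followed by SectionLength fence panel instances at fixed spacing.
; One more pillar is added after the loop, and both pieces use instanced static mesh components.
; The event graph has no active logic.
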(event EventBeginPlay)

(event Collision|EventActorBeginOverlap
  (params (OtherActor :type Actor%20Object%20Reference)))

(event EventTick
  (params (DeltaSeconds :type Float%20%28single-precision%29)))

(fn ConstructionScript
  (bind _pillarinstancedstaticmesh (Variables|Default|GetPillarInstancedStaticMesh))
  (for _index (range 1 (Variables|Default|GetSections%20Count))
    (Components|InstancedStaticMesh|AddInstance _pillarinstancedstaticmesh (Math|Transform|MakeTransform (Math|Vector|MakeVector 0.0 (* (- _index 1) (+ (* (Variables|Default|GetSection%20Length) 3e+02) 9e+01)) 0.0) "0, 0, 0" "1,1,1"))
    (for _index_2 (range 1 (Variables|Default|GetSection%20Length))
      (Components|InstancedStaticMesh|AddInstance (Variables|Default|GetFenceInstancedStaticMesh) (Math|Transform|MakeTransform (Math|Vector|MakeVector 0.0 (+ (* _index_2 3e+02) 305.0 (* (- _index 1) (+ (* (Variables|Default|GetSection%20Length) 3e+02) 9e+01))) 1.4e+02) "0, 0, 0" "1,1,1"))))
  (Components|InstancedStaticMesh|AddInstance _pillarinstancedstaticmesh (Math|Transform|MakeTransform (Math|Vector|MakeVector 0.0 (* (- _index 1) (+ (* (Variables|Default|GetSection%20Length) 3e+02) 9e+01)) 0.0) "0, 0, 0" "1,1,1")))